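; AI controller for a stealth enemy that turns perception events into Unaware, Chase and Search states.
; On possess it sets up the BB_StealthAI blackboard as Unaware; no behavior tree is started here.
; Perception updates branch on stimulus tag: Sight records the target and location for Chase, Hearing records the noise location for Search.
; Any lost stimulus clears player visibility, stores the last known location and switches to Search.
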(event OnTargetPerceptionUpdated(AIPerception)
  (params (Actor :type Actor%20Object%20Reference) (Stimulus :type AI%20Stimulus%20Structure))
  (bind (_age _expirationage _strength _stimuluslocation _receiverlocation _tag _bsuccessfullysensed) (Utilities|Struct|BreakAIStimulus Stimulus))
  (bind _returnvalue (AI|GetBlackboard 0))
  (bind _returnvalue_2 (AI|GetBlackboard 0))
  (bind _returnvalue_3 (AI|GetBlackboard 0))
  (if _bsuccessfullysensed
    ;[0.15 0.15 0.15 0.5] If Seen
    (if (== _tag "Sight")
      (AI|Components|Blackboard|SetValueasBool _returnvalue (Utilities|Name|MakeLiteralName "CanSeePlayer") true)
      (AI|Components|Blackboard|SetValueasObject _returnvalue (Utilities|Name|MakeLiteralName "TargetActor") Actor)
      (AI|Components|Blackboard|SetValueasVector _returnvalue (Utilities|Name|MakeLiteralName "LastKnownLocation") (Transformation|GetActorLocation Actor))
      (Class|BlackboardComponent|SetValueasString _returnvalue (Utilities|Name|MakeLiteralName "AIState") "Chase")
      (else
        ;[0.15 0.15 0.15 0.5] If Heard
        (if (== _tag "Hearing")
          (AI|Components|Blackboard|SetValueasBool _returnvalue_2 (Utilities|Name|MakeLiteralName "HeardNoise") true)
          (AI|Components|Blackboard|SetValueasVector _returnvalue_2 (Utilities|Name|MakeLiteralName "SearchLocation") _stimuluslocation)
          (Class|BlackboardComponent|SetValueasString _returnvalue_2 (Utilities|Name|MakeLiteralName "AIState") "Search"))))
    (else
      (AI|Components|Blackboard|SetValueasBool _returnvalue_3 (Utilities|Name|MakeLiteralName "CanSeePlayer") false)
      (Class|BlackboardComponent|SetValueasString _returnvalue_3 (Utilities|Name|MakeLiteralName "AIState") "Search")
      (AI|Components|Blackboard|SetValueasVector _returnvalue_3 (Utilities|Name|MakeLiteralName "LastKnownLocation") _stimuluslocation))))

(event EventBeginPlay)

(event EventTick
  (params (DeltaSeconds :type Float%20%28single-precision%29)))

(event EventPossess
  (params (PossessedPawn :type Pawn%20Object%20Reference))
  (bind _blackboardcomponent (Class|AIController|UseBlackboard "/Game/Enemy/AIEnemy/Blackboards/BB_StealthAI.BB_StealthAI"))
  (Class|BlackboardComponent|SetValueasString _blackboardcomponent (Utilities|Name|MakeLiteralName "AIState") "Unaware"))

(fn ConstructionScript)