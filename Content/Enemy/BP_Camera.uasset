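; Stealth security camera that sweeps in a sine arc and turns toward the player, within yaw limits, once sighted by its vision cone or pawn sensor.
; Tick raises or decays a suspicion meter, driving Unaware, Suspicious and Alert states that recolor the status light and update BP_StealthGameState.
; A rock or camera hit disables it, destroying the cone and dropping the head.
; Interact events let the player carry and throw the head.
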(event OnComponentBeginOverlap(Box)
  (params (OverlappedComponent :type Primitive%20Component%20Object%20Reference) (OtherActor :type Actor%20Object%20Reference) (OtherComp :type Primitive%20Component%20Object%20Reference) (OtherBodyIndex :type Integer) (bFromSweep :type Boolean) (SweepResult :type Hit%20Result%20Structure%20%28by%20ref%29))
  ;[0.15 0.15 0.15 0.5] Collision
  (Utilities|Casting|CastToBP_Rock OtherActor
    (:then
      _)
    (:CastFailed
      (Utilities|Casting|CastToBP_Camera OtherActor)))
  (Variables|Default|SetFunctional false)
  (CallFunction|StatusCheck))

(event OnComponentBeginOverlap(Cone)
  (params (OverlappedComponent :type Primitive%20Component%20Object%20Reference) (OtherActor :type Actor%20Object%20Reference) (OtherComp :type Primitive%20Component%20Object%20Reference) (OtherBodyIndex :type Integer) (bFromSweep :type Boolean) (SweepResult :type Hit%20Result%20Structure%20%28by%20ref%29))
  ;[0.15 0.15 0.15 0.5] Begin overlap with player character
  (Utilities|Casting|CastToBP_ThirdPersonCharacter OtherActor)
  (Variables|Default|SetbPlayerInSight true)
  (CallFunction|FollowPlayer))

(event OnComponentEndOverlap(Cone)
  (params (OverlappedComponent :type Primitive%20Component%20Object%20Reference) (OtherActor :type Actor%20Object%20Reference) (OtherComp :type Primitive%20Component%20Object%20Reference) (OtherBodyIndex :type Integer))
  ;[0.15 0.15 0.15 0.5] End overlap with player character
  (Utilities|Casting|CastToBP_ThirdPersonCharacter OtherActor)
  (Variables|Default|SetbPlayerInSight false))

(event OnSeePawn(PawnSensor)
  (params (Pawn :type Pawn%20Object%20Reference))
  (CallFunction|HandlePawnSighted Pawn))

(event Custom|Death
  ;[0.15 0.15 0.15 0.5] Death Sequence
  (Physics|SetSimulatePhysics (Variables|Default|GetCameraHead) true)
  (Rendering|Material|SetVectorParameterValue (Variables|Default|GetLightColor) "StatusLight" (Utilities|Struct|MakeLinearColor 0.0 0.0 0.0 1.0) :!class /Script/Engine.MaterialInstanceDynamic))

(event Custom|StatusCheck
  (bind _cone (Variables|Default|GetCone))
  ;[0.15 0.15 0.15 0.5] Rotation animation. Should stop and follow player but currently does not.
  (if (not (Variables|Default|GetFunctional))
    (if (Utilities|IsValid _cone)
      (Components|DestroyComponent _cone)
      (CallFunction|Death))))

(event Custom|HandlePawnSighted
  (params (SeenPawn :type Actor%20Object%20Reference))
  (Utilities|Casting|CastToBP_ThirdPersonCharacter SeenPawn)
  (Variables|Default|SetbPlayerInSight true)
  (Variables|Default|SetDetectedPlayer SeenPawn))

(event Custom|UpdateSuspicion
  (bind _suspicionmeter (Variables|Default|GetSuspicionMeter))
  ;[0.15 0.15 0.15 0.5] Suspicion meter system
  (if (>= _suspicionmeter 0.3)
    (CallFunction|SetCameraAlertState "NewEnumerator2")
    (elif (>= _suspicionmeter 0.1)
      (CallFunction|SetCameraAlertState "NewEnumerator1")
      (elif (<= _suspicionmeter 0.0)
        (CallFunction|SetCameraAlertState "NewEnumerator0")))))

(event Custom|SetCameraAlertState
  (params (NewState :type E_AlertState%20Enum :default "NewEnumerator0"))
  ;[0.15 0.15 0.15 0.5] New light correcting code that changes based on current state
  (if (Utilities|Enum|NotEqual(Enum) NewState (Variables|Default|GetCurrentCamState))
    (bind _output_get (Variables|Default|SetCurrentCamState NewState))
    (switch Utilities|FlowControl|Switch|SwitchonE_AlertState _output_get
      (:NewEnumerator0
        (Rendering|Material|SetVectorParameterValue (Variables|Default|GetLightColor) "StatusLight" (Utilities|Struct|MakeLinearColor 0.0 1.0 0.0 1.0) :!class /Script/Engine.MaterialInstanceDynamic))
      (:NewEnumerator1
        (Rendering|Material|SetVectorParameterValue (Variables|Default|GetLightColor) "StatusLight" (Utilities|Struct|MakeLinearColor 1.0 1.0 0.0 1.0) :!class /Script/Engine.MaterialInstanceDynamic))
      (:NewEnumerator2
        (Rendering|Material|SetVectorParameterValue (Variables|Default|GetLightColor) "StatusLight" (Utilities|Struct|MakeLinearColor 1.0 0.0 0.0 1.0) :!class /Script/Engine.MaterialInstanceDynamic)))
    (bind _asbp_stealth_game_state (Utilities|Casting|CastToBP_StealthGameState (Game|GetGameState)))
    (Default|UpdateAlertState _asbp_stealth_game_state NewState)))

(event Custom|FollowPlayer)

(event Custom|Sweep
  (if (Variables|Default|GetFunctional)
    _))

(event EventBeginPlay
  (bind _arrow (Variables|Default|GetArrow))
  (bind _returnvalue (Transformation|GetWorldRotation _arrow))
  ;[0.15 0.15 0.15 0.5] Sets current function status and light color upon creation
  (Variables|Default|SetFunctional true)
  (CallFunction|StatusCheck)
  (CallFunction|SetCameraAlertState "NewEnumerator0")
  (Rendering|Material|SetVectorParameterValue (Variables|Default|GetLightColor) "StatusLight" (Utilities|Struct|MakeLinearColor 0.0 1.0 0.0 1.0) :!class /Script/Engine.MaterialInstanceDynamic)
  (Variables|Default|SetInitialYaw (.yaw _returnvalue))
  (Variables|Default|SetInitialPitch (.pitch _returnvalue))
  (Variables|Default|SetInitialRoll (.roll _returnvalue)))

(event EventTick
  (params (DeltaSeconds :type Float%20%28single-precision%29))
  (bind _bplayerinsight (Variables|Default|GetbPlayerInSight))
  (bind _initialyaw (Variables|Default|GetInitialYaw))
  (bind _arrow (Variables|Default|GetArrow))
  (bind _initialroll (Variables|Default|GetInitialRoll))
  (bind _initialpitch (Variables|Default|GetInitialPitch))
  ;[0.15 0.15 0.15 0.5] Tick//Handles suspicion meter math
  ;;[0.15 0.15 0.15 0.5] Suspicion meter math (clamped to 0 - 1)
  (if _bplayerinsight
    (Variables|Default|SetInterpSpeed 5.0)
    (Variables|Default|SetSuspicionMeter (Math|Float|Clamp(Float) (+ (* (Variables|Default|GetSuspicionRate) DeltaSeconds) (Variables|Default|GetSuspicionMeter))))
    (else
      (Variables|Default|SetInterpSpeed 2.0)
      (Variables|Default|SetSuspicionMeter (Math|Float|Clamp(Float) (- (Variables|Default|GetSuspicionMeter) (* (Variables|Default|GetSuspicionRate) 0.5 DeltaSeconds))))))
  (Utilities|IsValid _arrow
    (:Is%20Valid
      (Transformation|SetWorldRotation _arrow (Math|Interpolation|RInterpTo (Transformation|GetWorldRotation (Variables|Default|GetArrow)) (Math|Rotator|SelectRotator (Math|Rotator|MakeRotator _initialroll _initialpitch (Math|Float|ClampAngle (.yaw (Math|Rotator|FindLookatRotation (Transformation|GetWorldLocation (Variables|Default|GetArrow)) (Transformation|GetActorLocation (Game|GetPlayerCharacter 0)))) (- _initialyaw 6e+01) (+ _initialyaw 6e+01))) (Math|Rotator|MakeRotator _initialroll _initialpitch (+ (* (Math|Trig|Sin(Radians) (* (Utilities|Time|GetGameTimeinSeconds) (Variables|Default|GetSweepSpeed))) (Variables|Default|GetMaxYaw)) (Variables|Default|GetInitialYaw))) _bplayerinsight) DeltaSeconds (Variables|Default|GetInterpSpeed)) false false)
      (CallFunction|UpdateSuspicion))))

(event EventINTInteract
  (params (PlayerRef :type BP%20Third%20Person%20Character%20Object%20Reference))
  (bind _camerahead (Variables|Default|GetCameraHead))
  ;[0.15 0.15 0.15 0.5] Pick up and Throw
  (if (not (Variables|/Game/ThirdPerson/Blueprints/BP_ThirdPersonCharacter.BP_ThirdPersonCharacter_C|GetbIsHolding PlayerRef))
    (Variables|/Game/ThirdPerson/Blueprints/BP_ThirdPersonCharacter.BP_ThirdPersonCharacter_C|SetbIsHolding PlayerRef true)
    (Variables|/Game/ThirdPerson/Blueprints/BP_ThirdPersonCharacter.BP_ThirdPersonCharacter_C|SetThrowable PlayerRef true)
    (Physics|SetSimulatePhysics _camerahead false)
    (Collision|SetCollisionEnabled _camerahead "NoCollision")
    (Transformation|AttachComponentToComponent (Variables|Default|GetCameraHead) (Variables|/Game/ThirdPerson/Blueprints/BP_ThirdPersonCharacter.BP_ThirdPersonCharacter_C|GetArrow1 PlayerRef) "None" "SnapToTarget" "KeepRelative" "KeepRelative" false)))

(event EventINTThrow
  (params (PlayerRef :type BP%20Third%20Person%20Character%20Object%20Reference))
  (bind _camerahead (Variables|Default|GetCameraHead))
  ;[0.15 0.15 0.15 0.5] Pick up and Throw
  (Physics|SetSimulatePhysics _camerahead true)
  (Collision|SetCollisionEnabled _camerahead "QueryAndPhysics")
  (Transformation|DetachFromComponent _camerahead "KeepWorld" "KeepWorld" "KeepWorld" true)
  (Physics|AddImpulse (Variables|Default|GetCameraHead) (* (Math|Vector|GetForwardVector (Variables|/Game/ThirdPerson/Blueprints/BP_ThirdPersonCharacter.BP_ThirdPersonCharacter_C|GetArrow1 PlayerRef)) 1500) "None" true))

(fn ConstructionScript
  (bind _returnvalue (Rendering|Material|CreateDynamicMaterialInstance (Variables|Default|GetLight) 0 "/Game/Interactables/Animated/ButtonMaterials/M_ButtonLight.M_ButtonLight" "None" :!class /Script/Engine.PrimitiveComponent))
  (bind _output_get (Variables|Default|SetLightColor _returnvalue))
  (Rendering|Material|SetVectorParameterValue :self _output_get :ParameterName "StatusLight" :!class /Script/Engine.MaterialInstanceDynamic))