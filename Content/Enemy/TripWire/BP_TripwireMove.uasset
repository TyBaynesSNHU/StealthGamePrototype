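; Moving tripwire laser hazard that fails the player on contact.
; On BeginPlay, the Movement timeline lerps the Cylinder's relative Z location up to 250 units above its start position.
; A Box overlap with BP_ThirdPersonCharacter clears that character's WinCondition and calls its FailState.
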(event OnComponentBeginOverlap(Box)
  (params (OverlappedComponent :type Primitive%20Component%20Object%20Reference) (OtherActor :type Actor%20Object%20Reference) (OtherComp :type Primitive%20Component%20Object%20Reference) (OtherBodyIndex :type Integer) (bFromSweep :type Boolean) (SweepResult :type Hit%20Result%20Structure%20%28by%20ref%29))
  ;[0.15 0.15 0.15 0.5] On overlap, run FailState on PlayerChar
  (bind _asbp_third_person_character (Utilities|Casting|CastToBP_ThirdPersonCharacter OtherActor))
  (Variables|/Game/ThirdPerson/Blueprints/BP_ThirdPersonCharacter.BP_ThirdPersonCharacter_C|SetWinCondition _asbp_third_person_character false)
  (Default|FailState _asbp_third_person_character))

(event EventBeginPlay
  ;[0.15 0.15 0.15 0.5] Moves laser back and fourth
  (Variables|Default|SetStartLocation (Variables|/Script/Engine.SceneComponent|GetRelativeLocation (Variables|Default|GetCylinder)))
  (bind _pos (Timeline|Movement Play)
    (:Update
      (Transformation|SetRelativeLocation (Variables|Default|GetCylinder) (+ (Variables|Default|GetStartLocation) (Math|Vector|MakeVector 0.0 0.0 (Math|Float|Lerp 0.0 2.5e+02 _pos))) false false))))

(fn ConstructionScript)