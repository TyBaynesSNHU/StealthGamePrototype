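; BP_Turret is an enemy turret that uses AI perception to begin tracking and shooting at the player.
; Any perception update starts looping timers that aim the pivot at the player and spawn BP_TurretProjectile from ProjectileSpawn.
; Forgetting the player plays the VisionScan timeline to spin the pivot, but neither timer is ever cleared.
; An older line-trace visibility check remains but never runs.
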(event OnTargetPerceptionUpdated(AIPerception)
  (params (Actor :type Actor%20Object%20Reference) (Stimulus :type AI%20Stimulus%20Structure))
  ;[0.15 0.15 0.15 0.5] AI_Sight
  (bind _returnvalue (Class|AIPerceptionSystem|GetSenseClassforStimulus Stimulus))
  (Development|PrintString (Utilities|GetClassDisplayName _returnvalue))
  (Utilities|Time|SetTimerbyFunctionName 0 "FollowPlayer" 0.05 true)
  (Utilities|Time|SetTimerbyFunctionName 0 "fireAtPlayer" 0.5 true))

(event OnTargetPerceptionForgotten(AIPerception)
  (params (Actor :type Actor%20Object%20Reference))
  ;[0.15 0.15 0.15 0.5] AI_Sight
  (Utilities|Casting|CastToBP_PlayerChar Actor)
  (CallFunction|SearchforPlayer))

(event Custom|FollowPlayer
  ;[0.15 0.15 0.15 0.5] Rotate pivot to follow player
  (Transformation|SetWorldRotation (Variables|Default|GetPivot) (Math|Rotator|FindLookatRotation (Transformation|GetActorLocation) (Transformation|GetActorLocation (Game|GetPlayerCharacter 0))) false false))

(event Custom|fireAtPlayer
  ;[0.15 0.15 0.15 0.5] Fire at player
  (Game|SpawnActorfromClass "/Game/Enemy/Turret/BP_TurretProjectile.BP_TurretProjectile_C" (Transformation|GetWorldTransform (Variables|Default|GetProjectileSpawn)) "Undefined" "MultiplyWithRoot" 0 0))

(event Custom|CheckPlayerSeen
  ;[1 0 0 0.5] Checks visilibity of player(NOT USED)
)

(event Custom|SearchForPlayer
  ;[0.15 0.01592 0 0.5] Rotating animation(not active)
  (bind _visionscan (Timeline|VisionScan Play)
    (:Update
      (Transformation|SetRelativeRotation (Variables|Default|GetPivot) (Math|Rotator|MakeRotator 0.0 0.0 (Math|Float|Lerp 0.0 3.6e+02 _visionscan)) false false))))

(fn ConstructionScript)