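; BP_AISentry is an enemy sentry turret that follows and fires at the player once AI perception updates.
; Any perception update starts looping timers that rotate Pivot toward the player and spawn BP_TurretProjectile; nothing here stops them.
; A BP_Rock overlapping Box disables it, detaching Sphere and Turret as physics debris.
; A dynamic eye material shows functional and alert state, though AlertStatus is never set here.
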(event OnTargetPerceptionUpdated(AIPerception)
  (params (Actor :type Actor%20Object%20Reference) (Stimulus :type AI%20Stimulus%20Structure))
  ;[0.15 0.15 0.15 0.5] AI_Sight
  (bind _returnvalue (Class|AIPerceptionSystem|GetSenseClassforStimulus Stimulus))
  (Development|PrintString (Utilities|GetClassDisplayName _returnvalue))
  (Utilities|Time|SetTimerbyFunctionName 0 "FollowPlayer" 0.05 true)
  (Utilities|Time|SetTimerbyFunctionName 0 "fireAtPlayer" 0.5 true))

(event OnTargetPerceptionForgotten(AIPerception)
  (params (Actor :type Actor%20Object%20Reference))
  ;[0.15 0.15 0.15 0.5] AI_Sight
  (Utilities|Casting|CastToBP_PlayerChar Actor))

(event OnComponentBeginOverlap(Box)
  (params (OverlappedComponent :type Primitive%20Component%20Object%20Reference) (OtherActor :type Actor%20Object%20Reference) (OtherComp :type Primitive%20Component%20Object%20Reference) (OtherBodyIndex :type Integer) (bFromSweep :type Boolean) (SweepResult :type Hit%20Result%20Structure%20%28by%20ref%29))
  ;[0.15 0.15 0.15 0.5] Collision
  (Utilities|Casting|CastToBP_Rock OtherActor)
  (if (Variables|Default|GetFunctional)
    (Variables|Default|SetFunctional false)
    (CallFunction|StatusCheck)))

(event Custom|UpdateEyeColor
  (bind _eyecolor (Variables|Default|GetEyeColor))
  ;[0.15 0.15 0.15 0.5] Eye Color
  (if (Variables|Default|GetFunctional)
    (if (Variables|Default|GetAlertStatus)
      (Rendering|Material|SetVectorParameterValue _eyecolor "EyeStatus" (Utilities|Struct|MakeLinearColor 1.0 0.0 0.0 1.0) :!class /Script/Engine.MaterialInstanceDynamic)
      (else
        (Rendering|Material|SetVectorParameterValue _eyecolor "EyeStatus" (Utilities|Struct|MakeLinearColor 0.0 1.0 0.0 1.0) :!class /Script/Engine.MaterialInstanceDynamic)))
    (else
      (Rendering|Material|SetVectorParameterValue _eyecolor "EyeStatus" (Utilities|Struct|MakeLinearColor 0.0 0.0 0.0 1.0) :!class /Script/Engine.MaterialInstanceDynamic))))

(event Custom|Death
  (bind _turret (Variables|Default|GetTurret))
  (bind _sphere (Variables|Default|GetSphere))
  ;[0.15 0.15 0.15 0.5] Death Sequence
  (CallFunction|UpdateEyeColor)
  (Transformation|DetachFromComponent (Variables|Default|GetDefaultSceneRoot) "KeepRelative" "KeepRelative" "KeepRelative" true)
  (Transformation|DetachFromComponent _sphere "KeepRelative" "KeepRelative" "KeepRelative" true)
  (Physics|SetSimulatePhysics _sphere true)
  (Transformation|DetachFromComponent _turret "KeepRelative" "KeepRelative" "KeepRelative" true)
  (Physics|SetSimulatePhysics _turret true))

(event Custom|fireAtPlayer
  ;[0.15 0.15 0.15 0.5] Fire at player
  (Game|SpawnActorfromClass "/Game/Enemy/Turret/BP_TurretProjectile.BP_TurretProjectile_C" (Transformation|GetWorldTransform (Variables|Default|GetProjectileSpawn)) "Undefined" "MultiplyWithRoot" 0 0))

(event Custom|FollowPlayer
  ;[0.15 0.15 0.15 0.5] Rotate pivot to follow player
  (Transformation|SetWorldRotation (Variables|Default|GetPivot) (Math|Rotator|FindLookatRotation (Transformation|GetActorLocation) (Transformation|GetActorLocation (Game|GetPlayerCharacter 0))) false false))

(event Custom|StatusCheck
  ;[0.15 0.15 0.15 0.5] Check status, if functional or not
  (if (not (Variables|Default|GetFunctional))
    (CallFunction|Death)))

(event EventBeginPlay
  ;[0.15 0.15 0.15 0.5] Sets current function status and light color upon creation
  (Variables|Default|SetFunctional true)
  (CallFunction|UpdateEyeColor))

(fn ConstructionScript
  ;[0.15 0.15 0.15 0.5] Dynamic color adjustment. Begins when actor is created.
  (bind _returnvalue (Rendering|Material|CreateDynamicMaterialInstance (Variables|Default|GetEye) 0 "/Engine/BasicShapes/M_SentryEye.M_SentryEye" "None" :!class /Script/Engine.PrimitiveComponent))
  (bind _output_get (Variables|Default|SetEyeColor _returnvalue))
  (Rendering|Material|SetVectorParameterValue :self _output_get :ParameterName "EyeStatus" :!class /Script/Engine.MaterialInstanceDynamic))