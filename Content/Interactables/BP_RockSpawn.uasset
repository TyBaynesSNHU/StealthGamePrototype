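; BP_RockSpawn is a spawner that places a BP_Rock at its root and replaces it when it is moved away.
; A looping half-second timer checks the current rock's distance and calls SpawnNewRock past a small threshold.
; SpawnNewRock tracks rocks in an array, destroying the oldest valid one beyond three.
; CheckRockPos clears CurrentRock after spawning the replacement, so later checks lose track of the new rock.
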(event Custom|SpawnNewRock
  (bind _spawnedrocks (Variables|Default|GetSpawnedRocks))
  (bind _spawnedrocks_2 (Variables|Default|GetSpawnedRocks))
  (bind _output (Utilities|Array|Get(acopy) _spawnedrocks_2))
  (bind _returnvalue (Game|SpawnActorfromClass "/Game/Interactables/BP_Rock.BP_Rock_C" (Transformation|GetWorldTransform (Variables|Default|GetDefaultSceneRoot)) "Undefined" "MultiplyWithRoot" 0 0))
  (bind _output_get (Variables|Default|SetCurrentRock _returnvalue))
  (Utilities|Array|Add _spawnedrocks _output_get)
  (if (> (Utilities|Array|Length _spawnedrocks) 3)
    (Utilities|IsValid _output
      (:Is%20Valid
        (Actor|DestroyActor _output)
        (Utilities|Array|RemoveIndex _spawnedrocks_2)))))

(event Custom|CheckRockPos
  (Utilities|IsValid (Variables|Default|GetCurrentRock)
    (:Is%20Valid
      (if (> (Math|Vector|VectorLength (- (Transformation|GetActorLocation (Variables|Default|GetCurrentRock)) (Transformation|GetWorldLocation (Variables|Default|GetDefaultSceneRoot)))) 1e+01)
        (CallFunction|SpawnNewRock)
        (Variables|Default|SetCurrentRock 0)))))

(event EventBeginPlay
  (CallFunction|SpawnNewRock)
  (Utilities|Time|SetTimerbyFunctionName 0 "CheckRockPos" 0.5 true))

(fn ConstructionScript)