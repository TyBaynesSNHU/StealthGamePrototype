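; BP_BreakableButton is a button that unlocks its TargetDoor, triggered either by interaction or by a physics-simulating BP_Rock overlapping its Box.
; Both triggers set ButtonStatus and play their own timeline, sliding the Cube along local Y.
; Each timeline update also refreshes the status light and sets IsUnlocked on a valid door.
; The light uses a dynamic material instance created at construction, red when inactive and green when pressed.
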(event OnComponentBeginOverlap(Box)
  (params (OverlappedComponent :type Primitive%20Component%20Object%20Reference) (OtherActor :type Actor%20Object%20Reference) (OtherComp :type Primitive%20Component%20Object%20Reference) (OtherBodyIndex :type Integer) (bFromSweep :type Boolean) (SweepResult :type Hit%20Result%20Structure%20%28by%20ref%29))
  (bind _targetdoor (Variables|Default|GetTargetDoor))
  ;[0.15 0.15 0.15 0.5] Collision
  (bind _asbp_rock (Utilities|Casting|CastToBP_Rock OtherActor))
  (if (Physics|IsSimulatingPhysics (Variables|/Game/Interactables/BP_Rock.BP_Rock_C|GetCube _asbp_rock) "None")
    (Variables|Default|SetButtonStatus true)
    (bind _alpha (Timeline|Alpha Play)
      (:Update
        (Transformation|SetRelativeLocation (Variables|Default|GetCube) (Math|Vector|MakeVector 0.0 (Math|Float|Lerp -56.0 0.0 _alpha) 0.0) false false)
        (CallFunction|UpdateLightColor)
        (Utilities|IsValid _targetdoor
          (:Is%20Valid
            (Variables|/Game/Interactables/Animated/BP_Door.BP_Door_C|SetisUnlocked _targetdoor true)))))))

(event Custom|UpdateLightColor
  (bind _lightcolor (Variables|Default|GetLightColor))
  ;[0.15 0.15 0.15 0.5] Light Color
  (if (Variables|Default|GetButtonStatus)
    (Rendering|Material|SetVectorParameterValue _lightcolor "StatusLight" (Utilities|Struct|MakeLinearColor 0.0 1.0 0.0 1.0) :!class /Script/Engine.MaterialInstanceDynamic)
    (else
      (Rendering|Material|SetVectorParameterValue _lightcolor "StatusLight" (Utilities|Struct|MakeLinearColor 1.0 0.0 0.0 1.0) :!class /Script/Engine.MaterialInstanceDynamic))))

(event EventBeginPlay
  ;[0.15 0.15 0.15 0.5] Begin Play
  (Variables|Default|SetButtonStatus false)
  (CallFunction|UpdateLightColor))

(event EventINTInteract
  (params (PlayerRef :type BP%20Third%20Person%20Character%20Object%20Reference))
  (bind _targetdoor (Variables|Default|GetTargetDoor))
  ;[0.15 0.15 0.15 0.5] Enabling engaging button with interaction
  (Variables|Default|SetButtonStatus true)
  (bind _alpha (Timeline|Timeline Play)
    (:Update
      (Transformation|SetRelativeLocation (Variables|Default|GetCube) (Math|Vector|MakeVector 0.0 (Math|Float|Lerp -56.0 0.0 _alpha) 0.0) false false)
      (CallFunction|UpdateLightColor)
      (Utilities|IsValid _targetdoor
        (:Is%20Valid
          (Variables|/Game/Interactables/Animated/BP_Door.BP_Door_C|SetisUnlocked _targetdoor true))))))

(fn ConstructionScript
  (bind _returnvalue (Rendering|Material|CreateDynamicMaterialInstance (Variables|Default|GetLight) 0 "/Game/Interactables/Animated/ButtonMaterials/M_ButtonLight.M_ButtonLight" "None" :!class /Script/Engine.PrimitiveComponent))
  (bind _output_get (Variables|Default|SetLightColor _returnvalue))
  (Rendering|Material|SetVectorParameterValue :self _output_get :ParameterName "StatusLight" :!class /Script/Engine.MaterialInstanceDynamic))