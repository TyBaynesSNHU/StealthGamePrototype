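; BP_DoorKeyCard is an interactable keycard door that opens only for a player holding the matching red, blue or green key.
; INTInteract checks the door's color flags against the player's key booleans, printing "Locked" on failure or toggling a Timeline forward and reverse via FlipFlop.
; The Timeline yaws the Arrow component, using a dot product to pick swing direction from the player's side.
; The construction script tints Cube with PickupColor through a dynamic material.
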(event EventBeginPlay)

(event Collision|EventActorBeginOverlap
  (params (OtherActor :type Actor%20Object%20Reference)))

(event EventINTInteract
  (params (PlayerRef :type BP%20Third%20Person%20Character%20Object%20Reference))
  ;[0.15 0.15 0.15 0.5] On interact, determines if door is unlocked based on the enum from the PC on if they have the keycard or not, and will adjust how it opens based on player location
  (if (Variables|Default|GetisRed)
    (if (Variables|/Game/ThirdPerson/Blueprints/BP_ThirdPersonCharacter.BP_ThirdPersonCharacter_C|GethasRedKey PlayerRef)
      (Utilities|FlowControl|FlipFlop :!label _label
        (:A
          (bind _returnvalue (CallFunction|UpdateDoorAngle PlayerRef))
          (bind _alpha (Timeline|Timeline Play)
            (:Update
              (Transformation|SetRelativeRotation (Variables|Default|GetArrow) (Math|Rotator|MakeRotator 0.0 0.0 (Math|Float|Lerp 0.0 _returnvalue _alpha)) false false))))
        (:B
          (Timeline|Timeline Reverse)))
      (else
        (Development|PrintString "Locked" :!label _label_2)))
    (elif (Variables|Default|GetisBlue)
      (if (Variables|/Game/ThirdPerson/Blueprints/BP_ThirdPersonCharacter.BP_ThirdPersonCharacter_C|GethasBlueKey PlayerRef)
        (goto _label)
        (else
          (goto _label_2)))
      (elif (Variables|Default|GetisGreen)
        (if (Variables|/Game/ThirdPerson/Blueprints/BP_ThirdPersonCharacter.BP_ThirdPersonCharacter_C|GethasGreenKey PlayerRef)
          (goto _label)
          (else
            (goto _label_2)))))))

(fn ConstructionScript
  ;[0.15 0.15 0.15 0.5] Dynamically changing color system with variable to link to.
  (bind _returnvalue (Rendering|Material|CreateDynamicMaterialInstance (Variables|Default|GetCube) 0 "/Game/Interactables/Mat_Color.Mat_Color" "None" :!class /Script/Engine.PrimitiveComponent))
  (bind _output_get (Variables|Default|SetColorDMI _returnvalue))
  (Rendering|Material|SetVectorParameterValue _output_get "Color" (Variables|Default|GetPickupColor) :!class /Script/Engine.MaterialInstanceDynamic))

(fn UpdateDoorAngle
  (params (self2 :type Actor%20Object%20Reference))
  (return (select (> (Math|Vector|DotProduct (Math|Vector|GetUnitDirection(Vector) (Transformation|GetActorLocation) (Transformation|GetActorLocation self2)) (Transformation|GetActorForwardVector)) 0.0) 9e+01 -9e+01)))