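; BP_Rock is an interactable rock that the player can pick up and throw.
; INTInteract checks that the player's hands are free, sets the holding and throwable flags, disables Cube physics and collision, and attaches to the player's Arrow1.
; INTThrow calls DetachFromActor on the player reference, restores Cube physics and collision, and launches it along Arrow1's forward vector with a mass-independent impulse.
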(event EventINTInteract
  (params (PlayerRef :type BP%20Third%20Person%20Character%20Object%20Reference))
  (bind _cube (Variables|Default|GetCube))
  (bind _arrow1 (Variables|/Game/ThirdPerson/Blueprints/BP_ThirdPersonCharacter.BP_ThirdPersonCharacter_C|GetArrow1 PlayerRef))
  ;[0.15 0.15 0.15 0.5] Pickup system. The variables determine whether the object is placed when or thrown when the mouse is clicked again.
  (if (not (Variables|/Game/ThirdPerson/Blueprints/BP_ThirdPersonCharacter.BP_ThirdPersonCharacter_C|GetbIsHolding PlayerRef))
    (Utilities|IsValid _arrow1
      (:Is%20Valid
        (Variables|/Game/ThirdPerson/Blueprints/BP_ThirdPersonCharacter.BP_ThirdPersonCharacter_C|SetbIsHolding PlayerRef true)
        (Variables|/Game/ThirdPerson/Blueprints/BP_ThirdPersonCharacter.BP_ThirdPersonCharacter_C|SetThrowable PlayerRef true)
        (Physics|SetSimulatePhysics _cube false)
        (Collision|SetCollisionEnabled _cube "NoCollision")
        (bind _returnvalue (Transformation|AttachComponentToComponent self _arrow1 "None" "SnapToTarget" "KeepRelative" "KeepRelative" false))
        (if _returnvalue
          (Development|PrintString "Attached"))))))

(event EventINTThrow
  (params (PlayerRef :type BP%20Third%20Person%20Character%20Object%20Reference))
  (bind _cube (Variables|Default|GetCube))
  ;[0.15 0.15 0.15 0.5] Throws item when mouse is clicked.
  (Transformation|DetachFromActor PlayerRef "KeepWorld" "KeepWorld" "KeepWorld")
  (Collision|SetCollisionEnabled _cube "QueryAndPhysics")
  (Physics|SetSimulatePhysics _cube true)
  (Physics|AddImpulse (Variables|Default|GetCube) (* (Math|Vector|GetForwardVector (Variables|/Game/ThirdPerson/Blueprints/BP_ThirdPersonCharacter.BP_ThirdPersonCharacter_C|GetArrow1 PlayerRef)) 1500) "None" true))

(fn ConstructionScript)