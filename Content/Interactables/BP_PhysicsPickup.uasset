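; BP_PhysicsPickup is an interactable physics cube meant to be held by the player, then dropped or thrown.
; INTDrop detaches the actor in world space and restores the cube's physics and collision.
; The pickup logic, which attaches the cube to the player's Arrow1 and sets holding flags, is disconnected, leaving INTInteract empty.
; The construction script's dynamic-material coloring from PickupColor is also disconnected.
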(event EventINTInteract
  (params (PlayerRef :type BP%20Third%20Person%20Character%20Object%20Reference))
  ;[0.15 0.15 0.15 0.5] Pickup system. The variables determine whether the object is placed when or thrown when the mouse is clicked again.
)

(event EventINTDrop
  (bind _cube (Variables|Default|GetCube))
  ;[0.15 0.15 0.15 0.5] Drops the held object based on current location of the player
  (Physics|SetSimulatePhysics _cube true)
  (Collision|SetCollisionEnabled _cube "QueryAndPhysics")
  (Transformation|DetachFromActor "KeepWorld" "KeepWorld" "KeepWorld"))

(fn ConstructionScript
  ;[0.15 0.15 0.15 0.5] Reattach to use: Dynamically changing color system
)